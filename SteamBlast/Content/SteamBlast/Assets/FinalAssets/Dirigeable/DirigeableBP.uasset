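; Airship (dirigeable) actor that travels along the spline of the Movementzepelin actor in the level.
; On BeginPlay it finds that actor and starts a timeline, with play rate set to the inverse of TimeToComplete.
; Each timeline update maps the track value to a distance along the spline and sets the airship's world location and rotation from that point.
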(event Custom|MoveZep
  (bind _splineref (Variables|Default|GetSplineREF))
  (bind _spline (Variables|/Game/SteamBlast/Assets/FinalAssets/Dirigeable/Movementzepelin.Movementzepelin_C|GetSpline _splineref))
  (Components|Timeline|SetPlayRate (Variables|Default|GetMove%20Object%20T) (/ 1.0 (Variables|Default|GetTimeToComplete)))
  (bind _movettrack (Timeline|Move%20Object%20T Play)
    (:Update
      (Transformation|SetActorTransform (Math|Transform|MakeTransform (Spline|GetLocationatDistanceAlongSpline _spline (Math|Float|Lerp 0.0 (Spline|GetSplineLength (Variables|/Game/SteamBlast/Assets/FinalAssets/Dirigeable/Movementzepelin.Movementzepelin_C|GetSpline (Variables|Default|GetSplineREF))) _movettrack) "World") (Spline|GetRotationatDistanceAlongSpline _spline (Math|Float|Lerp 0.0 (Spline|GetSplineLength (Variables|/Game/SteamBlast/Assets/FinalAssets/Dirigeable/Movementzepelin.Movementzepelin_C|GetSpline (Variables|Default|GetSplineREF))) _movettrack) "World") "1.000000,1.000000,1.000000")))))

(event EventBeginPlay
  (bind _returnvalue (Actor|GetActorOfClass "/Game/SteamBlast/Assets/FinalAssets/Dirigeable/Movementzepelin.Movementzepelin_C"))
  (Variables|Default|SetSplineREF _returnvalue)
  (CallFunction|MoveZep))

(fn ConstructionScript)