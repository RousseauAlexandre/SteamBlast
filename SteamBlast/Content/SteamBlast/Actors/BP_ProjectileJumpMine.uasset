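; BP_ProjectileJumpMine is the thrown form of the jump mine, launched with a given velocity at doubled time dilation while ignoring collision with the player.
; On impact, it spawns a BP_JumpMine aligned to the surface normal and destroys itself.
; Hitting another mine or mine projectile refunds the player's mine count instead.
; Actors with a BP_Metal component make it switch to physics simulation rather than deploy.
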(event Custom|Throw
  (params (Velocity :type Vector))
  (bind _returnvalue (Game|GetPlayerCharacter 0))
  (bind _self self)
  (bind _projectilemovement (Variables|Default|GetProjectileMovement))
  ;[1 1 1] Throw
  (Variables|/Script/Engine.MovementComponent|SetVelocity _projectilemovement Velocity)
  (Variables|Default|SetCustomTimeDilation _self 2.0)
  (Components|Activation|Activate _projectilemovement false)
  (Collision|IgnoreActorwhenMoving (Variables|Default|GetCube _self) _returnvalue true)
  (Collision|IgnoreActorwhenMoving (Variables|/Script/Engine.Character|GetCapsuleComponent _returnvalue) _self true))

(event EventBeginPlay)

(event Collision|EventActorBeginOverlap
  (params (OtherActor :type Actor%20Object%20Reference)))

(event EventTick
  (params (DeltaSeconds :type Float%20%28single-precision%29)))

(event Collision|EventHit
  (params (MyComp :type Primitive%20Component%20Object%20Reference) (Other :type Actor%20Object%20Reference) (OtherComp :type Primitive%20Component%20Object%20Reference) (bSelfMoved :type Boolean) (HitLocation :type Vector :default "0, 0, 0") (HitNormal :type Vector :default "0, 0, 0") (NormalImpulse :type Vector :default "0, 0, 0") (Hit :type Hit%20Result%20Structure%20%28by%20ref%29))
  (bind _returnvalue (Game|GetPlayerCharacter 0))
  (bind (_bblockinghit _binitialoverlap _time _distance _location _impactpoint _normal _impactnormal _physmat _hitactor) (Collision|BreakHitResult Hit))
  ;[1 1 1] Landing
  (if (!= _hitactor _returnvalue)
    (Utilities|Casting|CastToBP_JumpMine _hitactor
      (:then
        (bind _asbp_first_person_character (Utilities|Casting|CastToBP_FirstPersonCharacter _returnvalue :!label _label))
        (Variables|/Game/FirstPerson/Blueprints/BP_FirstPersonCharacter.BP_FirstPersonCharacter_C|SetMineAvalaible _asbp_first_person_character (+ (Variables|/Game/FirstPerson/Blueprints/BP_FirstPersonCharacter.BP_FirstPersonCharacter_C|GetMineAvalaible _asbp_first_person_character) 1))
        (Actor|DestroyActor))
      (:CastFailed
        (Utilities|Casting|CastToBP_ProjectileJumpMine _hitactor
          (:then
            (goto _label))
          (:CastFailed
            (Utilities|Casting|CastToBP_Metal (Actor|GetComponentbyClass _hitactor "/Game/SteamBlast/Actors/BP_Metal.BP_Metal_C")
              (:then
                (Physics|SetSimulatePhysics (Variables|Default|GetCube) true))
              (:CastFailed
                (Game|SpawnActorfromClass "/Game/SteamBlast/Actors/BP_JumpMine.BP_JumpMine_C" (Math|Transform|MakeTransform _impactpoint (Math|Rotator|MakeRotfromZ _normal)) "AdjustIfPossibleButAlwaysSpawn" 0 0)
                (Actor|DestroyActor)))))))))

(fn ConstructionScript)