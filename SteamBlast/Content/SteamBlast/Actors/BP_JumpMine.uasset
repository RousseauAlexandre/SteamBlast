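; BP_JumpMine is a jump pad mine that launches the player character along its up vector on overlap.
; Near-horizontal orientations substitute an upward component into the launch direction.
; The launch temporarily removes falling lateral friction and sets air control, then applies different fixed values after a short delay.
; Each new mine decrements every mine's life counter, including its own, so the oldest is destroyed and at most five remain.
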(event Custom|DecreaseLife
  ;[1 1 1] ControlNuberOfMines
  (Variables|Default|SetInstanceLife (- (Variables|Default|GetInstanceLife) 1))
  (if (<= (Variables|Default|GetInstanceLife) 0)
    (Actor|DestroyActor)))

(event EventBeginPlay
  ;[1 1 1] ControlNuberOfMines
  (Variables|Default|SetInstanceLife 6)
  (bind _outactors (Actor|GetAllActorsOfClass "BP_JumpMine_C"))
  (CallFunction|DecreaseLife _outactors))

(event Collision|EventActorBeginOverlap
  (params (OtherActor :type Actor%20Object%20Reference))
  (bind _returnvalue (Transformation|GetActorUpVector))
  (bind _returnvalue_2 (Game|GetPlayerCharacter 0))
  (bind _charactermovement (Variables|/Script/Engine.Character|GetCharacterMovement _returnvalue_2))
  ;[1 1 1] Launch Character
  (if (== OtherActor (Game|GetPlayerCharacter 0))
    (if (Math|Float|NearlyEqual(Float) (.z _returnvalue) 0.0 0.5)
      (Character|LaunchCharacter _returnvalue_2 (* (Math|Vector|MakeVector (.x _returnvalue) (.y _returnvalue) 0.6) 1.1e+03) true true)
      (else
        (Character|LaunchCharacter _returnvalue_2 (* (Transformation|GetActorUpVector) 1.1e+03) true true)))
    (Variables|/Script/Engine.CharacterMovementComponent|SetFallingLateralFriction _charactermovement 0.0)
    (Variables|/Script/Engine.CharacterMovementComponent|SetAirControl _charactermovement 0.8)
    (Utilities|FlowControl|Delay 0.8)
    (Variables|/Script/Engine.CharacterMovementComponent|SetAirControl _charactermovement 4.0)
    (Variables|/Script/Engine.CharacterMovementComponent|SetFallingLateralFriction _charactermovement 0.2)))

(event EventTick
  (params (DeltaSeconds :type Float%20%28single-precision%29)))

(fn ConstructionScript)

(fn NewFunction0)