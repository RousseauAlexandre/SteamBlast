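; BP_ProjectileJumpMine is a thrown projectile that deploys a BP_JumpMine where it lands.
; Throw launches its projectile movement at double time dilation and makes the cube and player capsule ignore each other.
; On hit, it becomes a BP_JumpMine aligned to the surface normal on flat upward surfaces or actors with a BP_Metal component.
; Otherwise its cube simulates physics, and any mine or mine projectile it strikes is destroyed.
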(event Custom|Throw
  (params (Velocity :type Vector))
  (bind _returnvalue (Game|GetPlayerCharacter 0))
  (bind _self self)
  (bind _projectilemovement (Variables|Default|GetProjectileMovement))
  ;[1 1 1] Throw
  (Variables|/Script/Engine.MovementComponent|SetVelocity _projectilemovement Velocity)
  (Variables|Default|SetCustomTimeDilation _self 2.0)
  (Components|Activation|Activate _projectilemovement false)
  (Collision|IgnoreActorwhenMoving (Variables|Default|GetCube _self) _returnvalue true)
  (Collision|IgnoreActorwhenMoving (Variables|/Script/Engine.Character|GetCapsuleComponent _returnvalue) _self true))

(event EventBeginPlay)

(event Collision|EventActorBeginOverlap
  (params (OtherActor :type Actor%20Object%20Reference)))

(event EventTick
  (params (DeltaSeconds :type Float%20%28single-precision%29)))

(event Collision|EventHit
  (params (MyComp :type Primitive%20Component%20Object%20Reference) (Other :type Actor%20Object%20Reference) (OtherComp :type Primitive%20Component%20Object%20Reference) (bSelfMoved :type Boolean) (HitLocation :type Vector :default "0, 0, 0") (HitNormal :type Vector :default "0, 0, 0") (NormalImpulse :type Vector :default "0, 0, 0") (Hit :type Hit%20Result%20Structure%20%28by%20ref%29))
  (bind (_bblockinghit _binitialoverlap _time _distance _location _impactpoint _normal _impactnormal _physmat _hitactor) (Collision|BreakHitResult Hit))
  (bind (_yaw _pitch) (Math|Vector|GetYawPitchfromVector _normal))
  ;[1 1 1] Landing
  (if (!= _hitactor (Game|GetPlayerCharacter 0))
    (bind _asbp_jump_mine (Utilities|Casting|CastToBP_JumpMine _hitactor)
      (:then
        (Actor|DestroyActor _asbp_jump_mine)
        (Physics|SetSimulatePhysics (Variables|Default|GetCube) true :!label _label))
      (:CastFailed
        (bind _asbp_projectile_jump_mine (Utilities|Casting|CastToBP_ProjectileJumpMine _hitactor)
          (:then
            (Actor|DestroyActor _asbp_projectile_jump_mine)
            (goto _label))
          (:CastFailed
            (if (and (Math|Float|NearlyEqual(Float) _yaw 0.0 0.1) (Math|Float|NearlyEqual(Float) _pitch 9e+01 0.1))
              _
              (else
                (Utilities|Casting|CastToBP_Metal (Actor|GetComponentbyClass _hitactor "/Game/SteamBlast/Actors/BP_Metal.BP_Metal_C")
                  (:then
                    _)
                  (:CastFailed
                    (goto _label)))))
            (Game|SpawnActorfromClass "/Game/SteamBlast/Actors/BP_JumpMine.BP_JumpMine_C" (Math|Transform|MakeTransform _impactpoint (Math|Rotator|MakeRotfromZ _normal)) "AdjustIfPossibleButAlwaysSpawn" 0 0)
            (Actor|DestroyActor)))))))

(fn ConstructionScript)